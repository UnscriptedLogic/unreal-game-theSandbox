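; Actor component that subtly tilts its owner's camera toward the mouse cursor while Enabled.
; BeginPlay caches the camera's base relative rotation; each Tick converts cursor position relative to viewport size into yaw and pitch offsets scaled by max tilts.
; The camera's relative rotation eases toward base plus offset with RInterpTo.
; Mouse Y is negated before centering, so pitch spans minus one to minus three times MaxPitchTilt.
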(event `self.ReceiveBeginPlay`
  (`self.Initialize`))

(event `self.ReceiveTick`
  (params (DeltaSeconds :type "Float (single-precision)"))
  (if (`self.Enabled`)
    (set `self.DeltaTime` DeltaSeconds)
    (`self.SubtleCameraTilt`)))

(fn `Initialize`
  (set `self.BaseRot` (`SceneComponent.RelativeRotation` (`Actor.GetComponentByClass` (`self.GetOwner`) "/Script/Engine.CameraComponent"))))

(fn `SubtleCameraTilt`
  (locals (NormalizedX :type "Float (double-precision)") (NormalizedY :type "Float (double-precision)") (PitchOffset :type "Float (double-precision)") (YawOffset :type "Float (double-precision)"))
  (bind (_returnvalue_x _returnvalue_y) (`KismetMathLibrary.BreakVector2D` (`WidgetLayoutLibrary.GetViewportSize`)))
  (bind (_locationx _locationy _returnvalue) (`PlayerController.GetMousePosition` (`GameplayStatics.GetPlayerController` 0)))
  (bind _returnvalue_2 (`Actor.GetComponentByClass` (`self.GetOwner`) "/Script/Engine.CameraComponent"))
  (bind _returnvalue_3 (* _returnvalue_y 0.5))
  (bind _returnvalue_4 (* _returnvalue_x 0.5))
  (if _returnvalue
    (set `local.NormalizedX` (/ (- _locationx _returnvalue_4) _returnvalue_4))
    (set `local.NormalizedY` (/ (- (* _locationy -1.0) _returnvalue_3) _returnvalue_3))
    (set `local.PitchOffset` (* (`local.NormalizedY`) (`self.MaxPitchTilt`)))
    (set `local.YawOffset` (* (`local.NormalizedX`) (`self.MaxYawTilt`)))
    (`SceneComponent.K2_SetRelativeRotation` _returnvalue_2 (`KismetMathLibrary.RInterpTo` (`SceneComponent.RelativeRotation` _returnvalue_2) (`KismetMathLibrary.MakeRotator` (.roll (`self.BaseRot`)) (+ (.pitch (`self.BaseRot`)) (`local.PitchOffset`)) (+ (.yaw (`self.BaseRot`)) (`local.YawOffset`))) (`self.DeltaTime`) 3.0) false false)))