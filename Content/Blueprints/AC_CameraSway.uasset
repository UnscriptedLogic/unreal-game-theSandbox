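; Actor component that sways its owner's camera with a continuous sine and cosine motion.
; BeginPlay caches the CameraComponent's relative transform, and Tick advances a time accumulator by both world delta and tick delta each frame.
; CameraSway feeds amplitude and frequency values into math expressions, offsetting the cached location on Z (sine) and Y (cosine).
; A roll value is also computed but never applied.
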(event EventBeginPlay
  (bind _output_get (Variables|Default|SetCameraComponent (Actor|GetComponentbyClass (Components|GetOwner) "/Script/Engine.CameraComponent")))
  (Variables|Default|SetBaseTransform (Transformation|GetRelativeTransform _output_get)))

(event EventTick
  (params (DeltaSeconds :type Float%20%28single-precision%29))
  (Variables|Default|SetDeltaTime (+ (Variables|Default|GetDeltaTime) (Utilities|Time|GetWorldDeltaSeconds) DeltaSeconds))
  (CallFunction|CameraSway (Variables|Default|GetXAmplitude) (Variables|Default|GetXFrequency) (Variables|Default|GetYAmplitude) (Variables|Default|GetYFrequency)))

(fn NewFunction)

(fn CameraSway
  (params (XAmplitude :type Float%20%28double-precision%29) (XFrequency :type Float%20%28double-precision%29) (YAmplitude :type Float%20%28double-precision%29) (YFrequency :type Float%20%28double-precision%29))
  (bind _basetransform (Variables|Default|GetBaseTransform))
  (bind _location (Math|Transform|BreakTransform _basetransform))
  (LocalVariables|SetNewX (|((sin(({B2343331-4006-CD32-075C-90A40467C671}*amplitude)))*frequency) XAmplitude XFrequency))
  (LocalVariables|SetNewY (|((cos(({B2343331-4006-CD32-075C-90A40467C671}*frequency)))*amplitude) YFrequency YAmplitude))
  (LocalVariables|SetNewRoll (|((sin(({B2343331-4006-CD32-075C-90A40467C671}*0.100000)))*2)))
  (Transformation|SetRelativeLocation (Variables|Default|GetCameraComponent) (Math|Vector|MakeVector (.x _location) (+ (.y _location) (LocalVariables|GetNewY)) (+ (.z _location) (LocalVariables|GetNewX))) false false))