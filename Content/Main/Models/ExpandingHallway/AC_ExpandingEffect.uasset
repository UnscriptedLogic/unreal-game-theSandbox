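; Component that animates an expanding hallway effect by scaling a supplied Context actor along a given direction.
; Initialize stores both and collapses the actor to near-zero scale on that axis, via a direction-masked vector from CalculateScale.
; ExpandEffect and ShrinkEffect wait briefly, then run eased scale tweens to full or collapsed size.
; A resettable DoOnce blocks overlapping expand calls, while shrinking first snaps to full scale.
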(event `Initialize`
  (params (Context :type "Actor Object Reference") (Direction :type "Vector Structure"))
  (set `self.Context` Context)
  (`self.Reset`)
  (set `self.Direction` Direction))

(event `ShrinkEffect`
  (bind _context (`self.Context`))
  (`Actor.SetActorRelativeScale3D` _context (1.0 1.0 1.0))
  (`KismetSystemLibrary.Delay` 1.0)
  (`XiTweenUtil.TweenActorLocalScaleSync` "ExpandingHallwayEffect" 2.0 _context (`self.CalculateScale`) "OutCubic"))

(event `ExpandEffect`
  (`/Engine/EditorBlueprintResources/StandardMacros.DoOnce` false :!label _label
    (:`Completed`
      (`KismetSystemLibrary.Delay` 1.0)
      (`XiTweenUtil.TweenActorLocalScaleSync` "ExpandingHallwayEffect" 2.0 (`self.Context`) (1.0 1.0 1.0) "OutSine")
      (`KismetSystemLibrary.Delay` 0.2)
      (goto _label :!via `Reset`))))

(event `Reset`
  (`Actor.SetActorRelativeScale3D` (`self.Context`) (`self.CalculateScale`)))

(fn `CalculateScale`
  (returns (ReturnValue :type "Vector Structure"))
  (bind _direction (`self.Direction`))
  (return (+ (- (`KismetMathLibrary.Vector_One`) _direction) (* _direction 0.001))))