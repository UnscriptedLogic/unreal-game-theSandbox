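; Game mode for multiplayer Pong that assigns player sides and spawns the ball.
; ChoosePlayerStart picks the "Right" start while the player list is empty, otherwise "Left".
; PostLogin adds each Pong player controller to that list and spawns a ball on every such login once it holds at least two.
; BeginPlay caches the Pong game state, which nothing else here uses.
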(event `self.ReceiveBeginPlay`
  (bind _asgs_pong_game_state (cast `/Game/Main/PongMultiplayer/GS_PongGameState` (`GameplayStatics.GetGameState`)))
  (set `self.PongGameState` _asgs_pong_game_state))

(event `self.K2_PostLogin`
  (params (NewPlayer :type "PlayerController Object Reference"))
  (bind _aspc_pong_multiplayer (cast `/Game/Main/PongMultiplayer/PC_PongMultiplayer` NewPlayer))
  (`KismetArrayLibrary.Array_Add` (`self.Players`) _aspc_pong_multiplayer)
  (if (>= (`KismetArrayLibrary.Array_Length` (`self.Players`)) 2)
    (`|SpawnActorFromClass` "/Game/Main/PongMultiplayer/A_PongBall.A_PongBall_C" (`KismetMathLibrary.MakeTransform` (0.0 0.0 0.0)) "Undefined" "MultiplyWithRoot" null null)))

(fn `ChoosePlayerStart`
  (params (Player :type "Controller Object Reference"))
  (returns (ReturnValue :type "Actor Object Reference"))
  (return (`self.K2_FindPlayerStart` Player (select `bool` (== (`KismetArrayLibrary.Array_Length` (`self.Players`)) 0) :`false` "Left" :`true` "Right"))))

(fn `UserConstructionScript`)