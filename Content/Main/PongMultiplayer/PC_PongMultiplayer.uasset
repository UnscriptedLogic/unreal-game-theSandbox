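; Player controller for the multiplayer Pong game that sets up local input, HUD and a shared camera view.
; On BeginPlay, the local controller caches its Pong player state, adds the default Enhanced Input mapping context, shows the cursor and creates the HUD widget.
; On possess it enables pawn input and switches the view to the first actor tagged SharedCamera; on unpossess it disables that input.
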(event `self.ReceiveBeginPlay`
  (if (`self.IsLocalController`)
    (`|ExecutionSequence`
      (:`then_0`
        (bind _asps_pong_player_state (cast `/Game/Main/PongMultiplayer/PS_PongPlayerState` (`GameplayStatics.GetPlayerState` 0)))
        (set `self.PongPlayerState` _asps_pong_player_state))
      (:`then_1`
        (`EnhancedInputSubsystemInterface.AddMappingContext` (subsystem `EnhancedInputLocalPlayerSubsystem`) "/Game/Main/Blueprints/FirstPerson/IMC_Default.IMC_Default" 0 (struct)))
      (:`then_2`
        (set `self.bShowMouseCursor` true))
      (:`then_3`
        (bind _returnvalue (`|CreateWidget` "/Game/Main/PongMultiplayer/WB_PongGameHUD.WB_PongGameHUD_C" self))
        (`UserWidget.AddToViewport` _returnvalue 0)))))

(event `self.ReceivePossess`
  (params (PossessedPawn :type "Pawn Object Reference"))
  (`self.EnableInput` PossessedPawn self)
  (bind _outactors (`GameplayStatics.GetAllActorsWithTag` "SharedCamera"))
  (if (> (`KismetArrayLibrary.Array_Length` _outactors) 0)
    (`self.SetViewTargetWithBlend` (`|GetArrayItem` _outactors))))

(event `self.ReceiveUnPossess`
  (params (UnpossessedPawn :type "Pawn Object Reference"))
  (`self.DisableInput` UnpossessedPawn self))

(fn `UserConstructionScript`)