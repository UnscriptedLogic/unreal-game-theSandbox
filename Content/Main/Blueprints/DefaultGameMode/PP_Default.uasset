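; PP_Default is a first-person player pawn built on a physics-driven Cube, with look and movement components.
; On possession its Arrow claims the CM_CameraManager camera; while claimed, look input yaws the Cube and pitches the Arrow.
; Each controlled tick sets velocity from the movement component, biasing Z downward by a fraction of its magnitude, and prints debug state.
; A downward line trace supplies grounding and gates the impulse-based jump.
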(event `self.ReceiveBeginPlay`
  (`|ExecutionSequence`
    (:`then_0`
      (set `/Game/Main/Blueprints/FirstPerson/AC_FPCameraLook.Ref` (`self.Arrow`) (`self.AC_FPCameraLook`))
      (`/Game/Main/Blueprints/FirstPerson/AC_FPMovement.Initialize` (`self.AC_FPMovement`) (`self.Cube`) (`self.Arrow`) (`self.Box`)))
    (:`then_1`
      (add `/Game/Main/Blueprints/FirstPerson/AC_FPMovement.OnJump_Event` (`self.AC_FPMovement`) (`|CreateDelegate` :!event `OnJump`)))))

(event `self.ReceivePossessed`
  (params (NewController :type "Controller Object Reference"))
  (`|ExecutionSequence`
    (:`then_0`
      (bind _ascm_camera_manager (cast `/Game/Main/Blueprints/DefaultGameMode/CM_CameraManager` (`GameplayStatics.GetPlayerCameraManager` 0)))
      (set `self.CM_CameraManager` _ascm_camera_manager))
    (:`then_1`
      (`/Game/Main/Blueprints/DefaultGameMode/CM_CameraManager.Claim` (`self.CM_CameraManager`) (`self.Arrow`)))))

(event `self.ReceiveTick`
  (params (DeltaSeconds :type "Float (single-precision)"))
  (bind (_grounded _hitactor _hitcomponent) (`self.GroundCheck`))
  (bind _cube (`self.Cube`))
  (bind _velocity (`/Game/Main/Blueprints/FirstPerson/AC_FPMovement.CalculateVelocity` (`self.AC_FPMovement`)))
  (bind (_lookdir_x _lookdir_y) (`KismetMathLibrary.BreakVector` (`/Game/Main/Blueprints/FirstPerson/AC_FPCameraLook.LookDir` (`self.AC_FPCameraLook`))))
  (`|ExecutionSequence`
    (:`then_0`
      (if (`/Game/Main/Blueprints/DefaultGameMode/CM_CameraManager.IsCurrentlyClaiming` (`self.CM_CameraManager`) (`self.Arrow`))
        (`SceneComponent.K2_AddLocalRotation` (`self.Cube`) (`KismetMathLibrary.MakeRotator` 0.0 0.0 _lookdir_x) false false)
        (`SceneComponent.K2_AddLocalRotation` (`self.Arrow`) (`KismetMathLibrary.MakeRotator` 0.0 _lookdir_y) false false)))
    (:`then_1`
      (`/Engine/EditorBlueprintResources/StandardMacros.IsValid` (`self.GetController`)
        (:`Is Valid`
          (bind _output_get (set `/Game/Main/Blueprints/FirstPerson/AC_FPMovement.IsGrounded` _grounded (`self.AC_FPMovement`)))
          (`KismetSystemLibrary.PrintString` (`KismetStringLibrary.Concat_StrStr` "[GROUNDED] Value: " (`KismetStringLibrary.Conv_BoolToString` _output_get) " | Grounded On: " (`KismetSystemLibrary.GetDisplayName` _hitactor) " With Component: " (`KismetSystemLibrary.GetDisplayName` _hitcomponent)) true true (struct :`R` 1.0 :`G` 0.806893 :`A` 1.0) 2.0 "PAWN.GROUNDED")
          (`KismetSystemLibrary.PrintString` (`KismetStringLibrary.Concat_StrStr` "[MOVEMENT] Calculated Velocity: " (`KismetStringLibrary.Conv_VectorToString` _velocity)) true true (struct :`R` 1.0 :`G` 0.482252 :`A` 1.0) 2.0 "PAWN.MOVEMENT")
          (bind _returnvalue (`PrimitiveComponent.GetPhysicsLinearVelocity` (`self.Cube`) "None"))
          (bind _z (.z _returnvalue))
          (`PrimitiveComponent.SetPhysicsLinearVelocity` _cube (+ (* (`SceneComponent.GetForwardVector` _cube) (.x _velocity)) (* (`SceneComponent.GetRightVector` _cube) (.y _velocity)) (`KismetMathLibrary.MakeVector` 0.0 0.0 (+ _z (* (`KismetMathLibrary.Abs` _z) -0.1)))) false "None"))))
    (:`then_2`)))

(event `OnJump`
  (if (`self.GroundCheck`)
    (`PrimitiveComponent.AddImpulse` (`self.Cube`) (`KismetMathLibrary.MakeVector` 0.0 0.0 (`self.JumpForce`)) "None" true)))

(fn `GroundCheck`
  (returns (Grounded :type Boolean) (HitActor :type "Actor Object Reference") (HitComponent :type "PrimitiveComponent Object Reference"))
  (bind _cube (`self.Cube`))
  (bind _relativelocation (`SceneComponent.RelativeLocation` _cube))
  (bind _outhit (`KismetSystemLibrary.LineTraceSingle` _relativelocation (+ _relativelocation (* (`SceneComponent.GetUpVector` _cube) -1.0 (`self.GroundCheckLength`))) "TraceTypeQuery1" false (`|MakeArray` self :!type "Actor Object Reference")))
  (bind (_bblockinghit _binitialoverlap _time _distance _location _impactpoint _normal _impactnormal _physmat _hitactor _hitcomponent) (`GameplayStatics.BreakHitResult` _outhit))
  (return (`KismetSystemLibrary.IsValid` _hitactor) _hitactor _hitcomponent))

(fn `UserConstructionScript`
  (bind _cube (`self.Cube`))
  (bind _relativelocation (`SceneComponent.RelativeLocation` _cube))
  (`KismetSystemLibrary.DrawDebugLine` _relativelocation (+ _relativelocation (* (`SceneComponent.GetUpVector` _cube) -1.0 175.0)) (struct :`R` 1.0 :`G` 0.073959 :`A` 1.0) 5.0 2.0))