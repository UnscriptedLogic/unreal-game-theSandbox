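; CM_CameraManager is a player camera manager that lets scene components claim control of the view.
; Claim inserts a component at the front of a list, so the newest claim wins, and Unclaim removes it, handing control back to the previous one.
; BlueprintUpdateCamera copies the front component's world location and rotation with a fixed FOV, overriding the default camera only while a claim exists.
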(fn `BlueprintUpdateCamera`
  (params (CameraTarget :type "Actor Object Reference"))
  (returns (NewCameraLocation :type "Vector Structure") (NewCameraRotation :type "Rotator Structure") (NewCameraFOV :type "Float (single-precision)") (ReturnValue :type Boolean))
  (bind (_valid _scenecomponent) (`self.HasValidClaimer`))
  (bind (_returnvalue_location _returnvalue_rotation) (`KismetMathLibrary.BreakTransform` (`SceneComponent.K2_GetComponentToWorld` _scenecomponent)))
  (if _valid
    (return _returnvalue_location _returnvalue_rotation 90.0 true)))

(fn `Claim`
  (params (Actor :type "SceneComponent Object Reference"))
  (bind _claims (`self.Claims`))
  (bind _actor (`local.Actor`))
  (if (not (`KismetArrayLibrary.Array_Contains` _claims _actor))
    (`KismetArrayLibrary.Array_Insert` _claims _actor)))

(fn `HasValidClaimer`
  (returns (Valid :type Boolean) (SceneComponent :type "SceneComponent Object Reference"))
  (bind _claims (`self.Claims`))
  (if (> (`KismetArrayLibrary.Array_Length` _claims) 0)
    (return true (`|GetArrayItem` _claims))
    (else
      (return false null))))

(fn `IsCurrentlyClaiming`
  (params (SceneComponent :type "SceneComponent Object Reference"))
  (returns (IsCurrentClaimer :type Boolean))
  (bind (_valid _scenecomponent) (`self.HasValidClaimer`))
  (`|ExecutionSequence`
    (:`then_0`
      (if _valid
        (if (== (`local.SceneComponent`) _scenecomponent)
          (return true))))
    (:`then_1`
      (return false))))

(fn `Unclaim`
  (params (Actor :type "SceneComponent Object Reference"))
  (if (`KismetArrayLibrary.Array_Contains` (`self.Claims`) (`local.Actor`))
    (`KismetArrayLibrary.Array_RemoveItem` (`self.Claims`) (`local.Actor`))))

(fn `UserConstructionScript`)