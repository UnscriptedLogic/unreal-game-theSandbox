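; GA_Test is a gameplay ability that spawns an actor of a configurable class where the avatar's camera is aimed.
; It uses the avatar's interaction component for a debug-drawn center-of-camera trace, offsetting the spawn from the hit along the surface normal.
; It then sends an AbilityTriggered gameplay event to the avatar with the spawned actor as payload, and ends immediately.
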(event `self.K2_ActivateAbility`
  (bind _returnvalue (`Actor.GetComponentByClass` (`self.GetAvatarActorFromActorInfo`) "/Game/Main/Blueprints/Components/Interaction/AC_InteractionComponent.AC_InteractionComponent_C"))
  (bind (_bblockinghit _hitactor _outhit) (`/Game/Main/Blueprints/Components/Interaction/AC_InteractionComponent.GetCenterOfCamera` :`self` _returnvalue :`DrawDebugType` "Persistent"))
  (bind (_bblockinghit_2 _binitialoverlap _time _distance _location _impactpoint _normal _impactnormal) (`GameplayStatics.BreakHitResult` _outhit))
  (`|ExecutionSequence`
    (:`then_0`
      (`/Engine/EditorBlueprintResources/StandardMacros.IsValid` _returnvalue
        (:`Is Valid`
          (if _bblockinghit
            (bind _returnvalue_2 (`|SpawnActorFromClass` (`self.ClassToSpawn`) (`KismetMathLibrary.MakeTransform` (+ _impactpoint (* _impactnormal 100.0))) "AdjustIfPossibleButAlwaysSpawn" "MultiplyWithRoot" null null))
            (`AbilitySystemBlueprintLibrary.SendGameplayEventToActor` (`self.GetAvatarActorFromActorInfo`) (struct :`TagName` "Event.AbilityTriggered") (make `GameplayEventData` (struct :`TagName` "Event.AbilityTriggered") null null _returnvalue_2))))))
    (:`then_1`
      (`self.K2_EndAbility`))))