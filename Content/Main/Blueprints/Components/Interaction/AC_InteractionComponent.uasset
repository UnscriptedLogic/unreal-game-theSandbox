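; Base interaction component that finds what a supplied camera is pointed at.
; Init stores the camera reference, and GetCenterOfCamera line-traces from it along its forward vector up to Range on the Visibility channel.
; The trace takes an ignore list and debug draw type and returns whether it hit, the actor and the full hit result.
; The Interact event is an empty stub with no logic of its own.
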(event `Init`
  (params (CameraRef :type "SceneComponent Object Reference"))
  (set `self.Camera Ref` CameraRef))

(event `self.Interact`)

(fn `GetCenterOfCamera`
  (params (ActorsToIgnore :type "Array of Actor Object Reference (by ref)") (DrawDebugType :type "EDrawDebugTrace Enum" :default "None"))
  (returns (bBlockingHit :type Boolean) (HitActor :type "Actor Object Reference") (OutHit :type "HitResult Structure"))
  (bind _camera_ref (`self.Camera Ref`))
  (bind _returnvalue (`SceneComponent.K2_GetComponentLocation` _camera_ref))
  (bind _outhit (`KismetSystemLibrary.LineTraceSingle` _returnvalue (+ _returnvalue (* (`KismetMathLibrary.GetForwardVector` (`SceneComponent.K2_GetComponentRotation` _camera_ref)) (`self.Range`))) "TraceTypeQuery1" false ActorsToIgnore DrawDebugType true (struct :`R` 1.0 :`A` 1.0) (struct :`G` 1.0 :`A` 1.0) 1.0))
  (bind (_bblockinghit _binitialoverlap _time _distance _location _impactpoint _normal _impactnormal _physmat _hitactor) (`GameplayStatics.BreakHitResult` _outhit))
  (return _bblockinghit _hitactor _outhit))