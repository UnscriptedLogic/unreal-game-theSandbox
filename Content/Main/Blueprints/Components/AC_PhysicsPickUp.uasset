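; Actor component that lets its owner pick up, carry and drop physics objects through a Physics Handle it adds on Init.
; Pick-up and let-go requests route to server events that grab at a location or release.
; UpdateHold moves the handle target to a hold point, auto-releasing beyond a maximum distance.
; On grab, an authority-only function scales handle stiffness, damping and interpolation by mass relative to max carry mass, so heavy objects lag.
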(event `Init`
  (bind _returnvalue (`|AddComponentByClass` (`self.GetOwner`) "/Script/Engine.PhysicsHandleComponent"))
  (set `self.PhysicsHandle` _returnvalue))

(event `TryPickUp`
  (params (Component :type "PrimitiveComponent Object Reference") (Location :type "Vector Structure"))
  (`self.Server_PickUp` Component Location))

(event `TryLetGo`
  (`self.Server_LetGo`))

(event `Server_PickUp`
  (params (Component :type "PrimitiveComponent Object Reference") (Location :type "Vector Structure"))
  (set `self.HeldComponent` Component)
  (`self.Server_AdjustForWeight`)
  (`PhysicsHandleComponent.GrabComponentAtLocation` (`self.PhysicsHandle`) Component "None" Location))

(event `UpdateHold`
  (params (HoldPoint :type "Vector Structure"))
  (`/Engine/EditorBlueprintResources/StandardMacros.IsValid` (`self.HeldComponent`)
    (:`Is Valid`
      (`|ExecutionSequence`
        (:`then_0`
          (`PhysicsHandleComponent.SetTargetLocation` (`self.PhysicsHandle`) HoldPoint))
        (:`then_1`
          (if (> (`KismetMathLibrary.Vector_Distance` (`SceneComponent.K2_GetComponentLocation` (`self.HeldComponent`)) HoldPoint) (`self.MaxDistance`))
            (`self.Server_LetGo`)))))))

(event `Server_LetGo`
  (`PhysicsHandleComponent.ReleaseComponent` (`self.PhysicsHandle`))
  (set `self.HeldComponent` null))

(fn `Server_AdjustForWeight`
  (locals (CalculatedStiffness :type "Float (single-precision)" :default 0.0) (WeightRatio :type "Float (single-precision)" :default 0.0))
  (`/Engine/EditorBlueprintResources/ActorComponentMacros.Switch Has Authority`
    (:`Authority`
      (`|ExecutionSequence`
        (:`then_0`
          (set `local.CalculatedStiffness` (`KismetMathLibrary.FClamp` (/ 12000.0 (`KismetMathLibrary.MultiplyMultiply_FloatFloat` (`PrimitiveComponent.GetMass` (`self.HeldComponent`)) 0.7)) 1200.0 12000.0))
          (set `local.WeightRatio` (`KismetMathLibrary.FClamp` (/ (`PrimitiveComponent.GetMass` (`self.HeldComponent`)) (`self.MaxCarryMass`)))))
        (:`then_1`
          (`PhysicsHandleComponent.SetLinearStiffness` (`self.PhysicsHandle`) (`KismetMathLibrary.Lerp` 12000.0 1500.0 (`local.WeightRatio`)))
          (`PhysicsHandleComponent.SetLinearDamping` (`self.PhysicsHandle`) (`KismetMathLibrary.Lerp` 200.0 700.0 (`local.WeightRatio`)))
          (`PhysicsHandleComponent.SetAngularStiffness` (`self.PhysicsHandle`) (`KismetMathLibrary.Lerp` 6000.0 800.0 (`local.WeightRatio`)))
          (`PhysicsHandleComponent.SetAngularDamping` (`self.PhysicsHandle`) (`KismetMathLibrary.Lerp` 200.0 900.0 (`local.WeightRatio`)))
          (`PhysicsHandleComponent.SetInterpolationSpeed` (`self.PhysicsHandle`) (`KismetMathLibrary.Lerp` 60.0 8.0 (`local.WeightRatio`))))))
    (:`Remote`
      (`KismetSystemLibrary.PrintString` "Server_AdjustForWeight was called on the client. This is a server function only"))))