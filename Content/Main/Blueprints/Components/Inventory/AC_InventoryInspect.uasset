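; Inventory inspection component that shows the currently selected item as a held actor attached to an anchor.
; Init binds inventory add/remove and index-change events, which all re-run InspectInventory at the stored index.
; InspectInventory clamps the index, clears the previous actor, then spawns the item's HeldActor from its ItemFrag_Inspectable fragment with relative offsets and fires inspect callbacks.
; TrySetInspect changes the index and returns a response code.
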(event `Init`
  (params (ActorAnchor :type "SceneComponent Object Reference") (Inventory :type "/Game/Main/Blueprints/Components/Inventory/Inventory Object Reference"))
  (bind _inventory (`self.Inventory`))
  (set `self.ActorAnchor` ActorAnchor)
  (`|ExecutionSequence`
    (:`then_0`
      (bind _output_get (set `self.Inventory` Inventory))
      (`/Engine/EditorBlueprintResources/StandardMacros.IsValid` _output_get
        (:`Is Valid`
          (add `InventoryBase.OnItemAdded` _inventory (`|CreateDelegate` :!event `OnItemAdded`))
          (add `InventoryBase.OnItemRemoved` _inventory (`|CreateDelegate` :!event `OnItemRemoved`))
          (add `self.OnInspectIndexChanged` (`|CreateDelegate` :!event `OnItemChanged`)))))))

(event `OnItemAdded`
  (params (Item :type "ItemBase Object Reference") (Inventory :type "InventoryBase Object Reference"))
  (`self.InspectInventory` (`self.InspectIndex`) Inventory))

(event `OnItemRemoved`
  (params (Item :type "ItemBase Object Reference") (Inventory :type "InventoryBase Object Reference"))
  (`self.InspectInventory` (`self.InspectIndex`) Inventory))

(event `OnItemChanged` :!signature `self.OnInspectIndexChanged`
  (params (Index :type Integer))
  (`self.InspectInventory` (`self.InspectIndex`) (`self.Inventory`)))

(fn `ClearInspect`
  (bind _held (`self.Held`))
  (`|ExecutionSequence`
    (:`then_0`
      (`/Engine/EditorBlueprintResources/StandardMacros.IsValid` (`self.CurrentInspectable`)
        (:`Is Valid`
          (`/Game/Main/Blueprints/Items/Fragments/ItemFrag_Inspectable.OnItemDeInspected` (`self.CurrentInspectable`)))))
    (:`then_1`
      (`/Engine/EditorBlueprintResources/StandardMacros.IsValid` _held
        (:`Is Valid`
          (`Actor.K2_DestroyActor` _held)
          (set `self.Held` null))))))

(fn `GetCurrentInspect`
  (returns (Item :type "ItemBase Object Reference"))
  (return (`|GetArrayItem` (`.items` (break `InventoryStruct` (`InventoryBase.data` (`self.Inventory`)))) (`self.InspectIndex`))))

(fn `InspectInventory`
  (params (Index :type Integer) (Inventory :type "InventoryBase Object Reference"))
  (bind _currentinspectable (`self.CurrentInspectable`))
  (bind _items (break `InventoryStruct` (`InventoryBase.data` (`local.Inventory`))))
  (bind (_fragment _returnvalue) (`ItemBase.HasFragment` (`|GetArrayItem` _items (`local.Index`)) "/Game/Main/Blueprints/Items/Fragments/ItemFrag_Inspectable.ItemFrag_Inspectable_C"))
  (set `self.InspectIndex` (`KismetMathLibrary.Clamp` Index 0 (`KismetArrayLibrary.Array_Length` (`.items` (break `InventoryStruct` (`InventoryBase.data` (`local.Inventory`)))))))
  (`self.ClearInspect`)
  (if (< (`self.InspectIndex`) (`KismetArrayLibrary.Array_Length` _items))
    (if _returnvalue
      (bind _asitem_frag_inspectable (cast `/Game/Main/Blueprints/Items/Fragments/ItemFrag_Inspectable` _fragment))
      (set `self.CurrentInspectable` _asitem_frag_inspectable)
      (`/Game/Main/Blueprints/Items/Fragments/ItemFrag_Inspectable.OnItemInspected` _currentinspectable)
      (bind _data (`/Game/Main/Blueprints/Items/Fragments/ItemFrag_Inspectable.GetInspectableData` _currentinspectable))
      (bind _returnvalue_2 (`|SpawnActorFromClass` (`/Game/Main/Blueprints/Items/InspectableDataAsset.HeldActor` _data) (`KismetMathLibrary.MakeTransform` (+ (`SceneComponent.RelativeLocation` (`self.ActorAnchor`)) (`/Game/Main/Blueprints/Items/InspectableDataAsset.RelativeLocationOffset` _data)) (`KismetMathLibrary.Conv_VectorToRotator` (`/Game/Main/Blueprints/Items/InspectableDataAsset.RelativeRotationOffset` _data)) (`/Game/Main/Blueprints/Items/InspectableDataAsset.RelativeScale` _data)) "AlwaysSpawn" "MultiplyWithRoot" null null))
      (set `self.Held` _returnvalue_2)
      (`Actor.K2_AttachToComponent` _returnvalue_2 (`self.ActorAnchor`) "None" "KeepRelative" "KeepRelative" "KeepRelative" true))))

(fn `IsInspectable`
  (returns (Value :type Boolean) (Inspectable :type "/Game/Main/Blueprints/Items/Fragments/ItemFrag_Inspectable Object Reference") (Item :type "ItemBase Object Reference"))
  (bind _output (`|GetArrayItem` (`.items` (break `InventoryStruct` (`InventoryBase.data` (`self.Inventory`)))) (`self.InspectIndex`)))
  (bind (_fragment _returnvalue) (`ItemBase.HasFragment` _output "/Game/Main/Blueprints/Items/Fragments/ItemFrag_Inspectable.ItemFrag_Inspectable_C"))
  (bind _asitem_frag_inspectable (cast `/Game/Main/Blueprints/Items/Fragments/ItemFrag_Inspectable` _fragment)
    (:`then`
      _)
    (:`CastFailed`
      _))
  (return _returnvalue _asitem_frag_inspectable _output))

(fn `TrySetInspect`
  (params (Index :type Integer))
  (returns (Response :type "Response Structure"))
  (bind _returnvalue (`KismetArrayLibrary.Array_Length` (`.items` (break `InventoryStruct` (`InventoryBase.data` (`self.Inventory`))))))
  (`|ExecutionSequence`
    (:`then_0`
      (if (> _returnvalue 0)
        (bind _output_get (set `self.InspectIndex` (`KismetMathLibrary.Clamp` (`local.Index`) 0 (- _returnvalue 0))))
        (`self.OnInspectIndexChanged` _output_get)
        (return (make `Response` 200))))
    (:`then_1`
      (return (make `Response` 500 "Internal Error")))))