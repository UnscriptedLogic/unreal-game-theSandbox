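; BP_WorldItem is a world representation of an item, displaying the static mesh from its item data.
; Its construction script calls Construct on ItemType when ItemObject is missing or of another class, then refreshes the mesh.
; UpdateItemMesh applies an already loaded mesh, async-loads an unloaded soft reference before updating again, or clears the mesh when ItemObject is invalid.
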(event `LoadItemMesh`
  (params (SoftRef :type "StaticMesh Soft Object Reference"))
  (`|LoadAsset` SoftRef
    (:`Completed`
      (`self.UpdateItemMesh`))))

(fn `UpdateItemMesh`
  (bind (_name _description _icon _mesh) (break `ItemStruct` (`ItemBase.ItemData` (`self.ItemObject`))))
  (bind _output (`|ConvertAsset` _mesh))
  (`self.ItemObject`
    (:`then`
      (`/Engine/EditorBlueprintResources/StandardMacros.IsValid` _output
        (:`Is Valid`
          (`StaticMeshComponent.SetStaticMesh` (`self.StaticMesh`) _output))
        (:`Is Not Valid`
          (`self.LoadItemMesh` _mesh))))
    (:`else`
      (`StaticMeshComponent.SetStaticMesh` (`self.StaticMesh`) null))))

(fn `UserConstructionScript`
  (`self.ItemType`
    (:`then`
      (bind _itemobject (`self.ItemObject`)
        (:`then`
          (if (not (== (`GameplayStatics.GetObjectClass` _itemobject) (`self.ItemType`)))
            (`|GenericCreateObject` (`self.ItemType`) :!label _label)
            (set `self.ItemObject` null)))
        (:`else`
          (goto _label)))
      (`self.UpdateItemMesh`))
    (:`else`)))