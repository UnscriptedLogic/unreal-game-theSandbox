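; Item component that makes its owner interactable through the fragments held in its item Data.
; On BeginPlay it passes Data to each fragment as context and binds interactable fragments' client and server interact events to its matching handlers.
; Those handlers relay the interactor through the component's own client and server events.
; It gathers non-empty prompts from fragments implementing IHasInteractMessage, while CanInteract always returns a 200 success response.
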(event `self.ReceiveBeginPlay`
  (for _array_element (`ItemBase.ItemFragments` (`self.Data`))
    (set `ItemFragment.itemContext` (`self.Data`) _array_element)
    (bind _asitem_frag_interactable (cast `/Game/Main/Blueprints/Items/Fragments/ItemFrag_Interactable` _array_element))
    (add `/Game/Main/Blueprints/Items/Fragments/ItemFrag_Interactable.OnClientInteract_Event` _asitem_frag_interactable (`|CreateDelegate` :!event `OnClientInteract`))
    (add `/Game/Main/Blueprints/Items/Fragments/ItemFrag_Interactable.OnServerInteract_Event` _asitem_frag_interactable (`|CreateDelegate` :!event `OnServerInteract`))))

(event `/Game/Main/Blueprints/Components/IInteractable.OnServerInteract`
  (params (Interactor :type "Actor Object Reference"))
  (`self.OnServerInteract_Event` Interactor))

(event `/Game/Main/Blueprints/Components/IInteractable.OnClientInteract`
  (params (Interactor :type "Actor Object Reference"))
  (`self.OnClientInteract_Event` Interactor))

(fn `CanInteract`
  (returns (Response :type "/Game/Main/Blueprints/Components/S_Response Structure"))
  (return (make `/Game/Main/Blueprints/Components/S_Response` 200)))

(fn `GetInteractionMessages`
  (returns (Messages :type "Array of String"))
  (locals (InteractionMessages :type "Array of String"))
  (for _array_element (`ItemBase.ItemFragments` (`self.Data`))
    (`/Engine/EditorBlueprintResources/StandardMacros.IsValid` _array_element
      (:`Is Valid`
        (bind _asihas_interact_message (cast `/Game/Main/Blueprints/Items/IHasInteractMessage` _array_element))
        (bind _desc (`/Game/Main/Blueprints/Items/IHasInteractMessage.GetInteractionMessage` _asihas_interact_message))
        (if (not (`KismetStringLibrary.IsEmpty` _desc))
          (`KismetArrayLibrary.Array_Add` (`local.InteractionMessages`) _desc)))))
  (return (`local.InteractionMessages`)))