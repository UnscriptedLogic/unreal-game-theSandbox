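; Actor component that plays footstep sounds while its owning Character walks on the ground with move input.
; It caches the owning Character on BeginPlay and stores the IA_Move value on trigger and completion.
; Tick runs a countdown while moving, playing the footstep cue at the owner's location with random volume each time the interval elapses.
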(event `self.ReceiveBeginPlay`
  (`|ExecutionSequence`
    (:`then_1`
      (bind _ascharacter (cast `Character` (`self.GetOwner`)))
      (`/Engine/EditorBlueprintResources/StandardMacros.IsValid` _ascharacter
        (:`Is Valid`
          (set `self.Character` _ascharacter))))))

(event `EnhancedInput|/Game/Main/Blueprints/FirstPerson/IA_Move`
  (params (ActionValue :type "Vector2D Structure") (ElapsedSeconds :type "Float (double-precision)") (TriggeredSeconds :type "Float (double-precision)") (InputAction :type "InputAction Object Reference" :default "/Game/Main/Blueprints/FirstPerson/IA_Move.IA_Move"))
  (:`Triggered`
    (set `self.Input` ActionValue :!label _label))
  (:`Completed`
    (goto _label)))

(event `self.ReceiveTick`
  (params (DeltaSeconds :type "Float (single-precision)"))
  (if (and (`NavMovementInterface.IsMovingOnGround` (`Character.CharacterMovement` (`self.Character`))) (> (`KismetMathLibrary.Abs` (`KismetMathLibrary.VSize2D` (`self.Input`))) 0.0))
    (if (<= (`self.Timer_Interval`) 0.0)
      (`GameplayStatics.PlaySoundAtLocation` "/Game/Main/Audio/Footsteps/Cue_Footsteps.Cue_Footsteps" (`Actor.K2_GetActorLocation` (`self.GetOwner`)) (struct) (`KismetMathLibrary.RandomFloatInRange` 0.25 0.75) 1.0 0.0 null null null null)
      (set `self.Timer_Interval` (`self.FootstepsInterval`))
      (else
        (set `self.Timer_Interval` (- (`self.Timer_Interval`) (`GameplayStatics.GetWorldDeltaSeconds`)))))))