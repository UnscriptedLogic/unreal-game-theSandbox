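; Actor component for client-priority physics pickup, carrying and release of objects through a physics handle it creates on its owner.
; Try events act locally, then call the server, toggling movement replication on any currently held object.
; Hold updates move the handle target and drop objects beyond a maximum distance.
; Pickup plays a sound and notifies item fragments; mass-based tuning is calculated, but fixed handle settings are applied.
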(event `Init`
  (bind _returnvalue (`|AddComponentByClass` (`self.GetOwner`) "/Script/Engine.PhysicsHandleComponent"))
  (set `self.PhysicsHandle` _returnvalue))

(event `TryPickUp`
  (params (Component :type "PrimitiveComponent Object Reference") (Location :type "Vector Structure") (HoldDistance :type "Float (double-precision)"))
  (`self.ToggleReplication` false)
  (`self.PickUp` Component Location HoldDistance)
  (`self.Server_PickUp` Component Location HoldDistance))

(event `TryLetGo`
  (`self.ToggleReplication` true)
  (`self.LetGo`)
  (`self.Server_LetGo`))

(event `TryUpdateHold`
  (params (HoldPoint :type "Vector Structure") (StartPoint :type "Vector Structure"))
  (`self.UpdateHold` HoldPoint)
  (`self.Server_UpdateHold` HoldPoint))

(event `LetGo`
  (`PhysicsHandleComponent.ReleaseComponent` (`self.PhysicsHandle`))
  (set `self.HeldComponent` null)
  (`self.OnLetGo`))

(event `UpdateHold`
  (params (HoldPoint :type "Vector Structure"))
  (`/Engine/EditorBlueprintResources/StandardMacros.IsValid` (`self.HeldComponent`)
    (:`Is Valid`
      (`|ExecutionSequence`
        (:`then_0`
          (`PhysicsHandleComponent.SetTargetLocation` (`self.PhysicsHandle`) HoldPoint))
        (:`then_1`
          (if (> (`KismetMathLibrary.Vector_Distance` (`SceneComponent.K2_GetComponentLocation` (`self.HeldComponent`)) HoldPoint) (`self.MaxDistance`))
            (`self.TryLetGo`)))))))

(event `PickUp`
  (params (Component :type "PrimitiveComponent Object Reference") (Location :type "Vector Structure") (InitialHoldLoc :type "Float (double-precision)"))
  (bind _returnvalue (`Actor.GetComponentByClass` (`self.GetOwner` Component) "/Game/Main/Blueprints/Components/Item/AC_ItemComponent.AC_ItemComponent_C"))
  (bind (_fragment _returnvalue_2) (`ItemBase.HasFragment` (`/Game/Main/Blueprints/Components/Item/AC_ItemComponent.Data` _returnvalue) "/Game/Main/Blueprints/Items/Fragments/ItemFrag_PhysicsPickUp.ItemFrag_PhysicsPickUp_C"))
  (`|ExecutionSequence`
    (:`then_0`
      (set `self.HoldDistance` InitialHoldLoc)
      (set `self.HeldComponent` Component)
      (`self.AdjustForWeight`)
      (`PhysicsHandleComponent.GrabComponentAtLocation` (`self.PhysicsHandle`) Component "None" Location))
    (:`then_1`
      (`/Engine/EditorBlueprintResources/StandardMacros.IsValid` _returnvalue
        (:`Is Valid`
          (if _returnvalue_2
            (bind _asitem_frag_physics_pick_up (cast `/Game/Main/Blueprints/Items/Fragments/ItemFrag_PhysicsPickUp` _fragment))
            (`/Game/Main/Blueprints/Items/Fragments/ItemFrag_PhysicsPickUp.OnPhysicsPickUp_Event` _asitem_frag_physics_pick_up)))))
    (:`then_2`
      (`GameplayStatics.PlaySoundAtLocation` "/Game/Main/Movers/SFX/PickUpSound.PickUpSound" (`Actor.K2_GetActorLocation` (`self.GetOwner`)) (struct) 1.0 1.0 0.0 "/Game/Main/ClassroomPurgatory/Blueprints/Misc/SA_Proximity.SA_Proximity" "/Game/Main/Movers/SFX/SC_MoversSoundConcurrency.SC_MoversSoundConcurrency" null null)
      (`self.OnPickedUp` Component Location))))

(event `Server_LetGo`
  (`self.LetGo`))

(event `Server_UpdateHold`
  (params (HoldPoint :type "Vector Structure"))
  (bind _actor (`self.Actor`))
  (`|ExecutionSequence`
    (:`then_0`
      (`self.UpdateHold` HoldPoint))
    (:`then_1`
      (`KismetSystemLibrary.Delay` 1.0)
      (`/Engine/EditorBlueprintResources/StandardMacros.IsValid` _actor
        (:`Is Valid`
          (bind _asa_furniture (cast `/Game/Main/Movers/Blueprints/Items/A_Furniture` _actor))
          (`/Game/Main/Movers/Blueprints/Items/A_Furniture.ReduceWeightTemporarily` _asa_furniture (`self.GetOwner`)))))))

(event `Server_PickUp`
  (params (Component :type "PrimitiveComponent Object Reference") (Location :type "Vector Structure") (InitialHoldLoc :type "Float (double-precision)"))
  (`self.PickUp` Component Location InitialHoldLoc))

(fn `AdjustForWeight`
  (locals (CalculatedStiffness :type "Float (single-precision)" :default 0.0) (WeightRatio :type "Float (single-precision)" :default 0.0))
  (`|ExecutionSequence`
    (:`then_0`
      (set `local.CalculatedStiffness` (`KismetMathLibrary.FClamp` (/ 12000.0 (`KismetMathLibrary.MultiplyMultiply_FloatFloat` (`PrimitiveComponent.GetMass` (`self.HeldComponent`)) 0.7)) 1200.0 12000.0))
      (set `local.WeightRatio` (`KismetMathLibrary.FClamp` (/ (`PrimitiveComponent.GetMass` (`self.HeldComponent`)) (`self.MaxCarryMass`)))))
    (:`then_2`
      (`PhysicsHandleComponent.SetLinearStiffness` (`self.PhysicsHandle`) 10000.0)
      (`PhysicsHandleComponent.SetLinearDamping` (`self.PhysicsHandle`) 10000.0)
      (`PhysicsHandleComponent.SetAngularStiffness` (`self.PhysicsHandle`) 10000.0)
      (`PhysicsHandleComponent.SetAngularDamping` (`self.PhysicsHandle`) 10000.0)
      (`PhysicsHandleComponent.SetInterpolationSpeed` (`self.PhysicsHandle`) 10.0))))

(fn `HasActive`
  (returns (ReturnValue :type Boolean))
  (return (`KismetSystemLibrary.IsValid` (`self.HeldComponent`))))

(fn `ToggleReplication`
  (params (Replicate :type Boolean))
  (bind _returnvalue (`self.GetOwner` (`self.HeldComponent`)))
  (`/Engine/EditorBlueprintResources/StandardMacros.IsValid` (`self.HeldComponent`)
    (:`Is Valid`
      (`Actor.SetReplicateMovement` _returnvalue Replicate)
      (if Replicate
        (`Actor.ForceNetUpdate` _returnvalue)))))