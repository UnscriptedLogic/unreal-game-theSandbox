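; Camera bobbing component that adds roll, FOV kicks, head bob and a landing dip to a supplied camera scene component.
; Move, look, jump and landing events nudge roll, FOV, bob amplitude or offset, mostly through a shared clamped accumulator.
; Tick eases these values back to rest with delta-scaled lerps, writing FOV to CM_CameraManager.
; A time-looped curve drives vertical bob; despite its name, OffsetPitch shifts height rather than pitch.
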(event `Init`
  (params (CameraSceneComponent :type "SceneComponent Object Reference"))
  (set `self.Camera Scene Component` CameraSceneComponent)
  (set `self.InitialTransform` (`SceneComponent.GetRelativeTransform` (`self.Camera Scene Component`)))
  (bind _ascm_camera_manager (cast `/Game/Main/Blueprints/DefaultGameMode/CM_CameraManager` (`GameplayStatics.GetPlayerCameraManager` 0)))
  (set `self.CameraManager` _ascm_camera_manager)
  (set `/Game/Main/Blueprints/DefaultGameMode/CM_CameraManager.FOV` (`self.DefaultFOV`) _ascm_camera_manager)
  (set `self.CurrentFOV` 120.0))

(event `LookRotation`
  (params (Input :type "Vector2D Structure"))
  (set `self.CurrentRoll` (`self.CalculateValueModify` Input_X)))

(event `JumpInput`
  (set `self.CurrentFOV` (+ (`self.CurrentFOV`) 1.0)))

(event `OnLanded`
  (set `self.OffsetPitch` -30.0))

(event `MoveInput`
  (params (Input :type "Vector2D Structure"))
  (bind _returnvalue (+ Input_X Input_Y))
  (set `self.CurrentRoll` (`self.CalculateValueModify` Input_X (`self.RollAcceleration`) (`self.CurrentRoll`) (`self.RollMax`)))
  (set `self.CurrentFOV` (`self.CalculateValueModify` (`KismetMathLibrary.NormalizeToRange` _returnvalue 0.0 1.0) (`self.RollAcceleration`) (`self.CurrentFOV`) 130.0))
  (set `self.BobAmplitude` (`self.CalculateValueModify` (`KismetMathLibrary.NormalizeToRange` _returnvalue 0.0 1.0) (`self.RollAcceleration`) (`self.BobAmplitude`) (`self.MaxBobHeight`))))

(event `self.ReceiveTick`
  (params (DeltaSeconds :type "Float (single-precision)"))
  (bind _camera_scene_component (`self.Camera Scene Component`))
  (bind _camera_scene_component_2 (`self.Camera Scene Component`))
  (bind (_relativelocation_x _relativelocation_y) (`KismetMathLibrary.BreakVector` (`SceneComponent.RelativeLocation` _camera_scene_component)))
  (bind (_relativerotation_roll _relativerotation_pitch _relativerotation_yaw) (`KismetMathLibrary.BreakRotator` (`SceneComponent.RelativeRotation` _camera_scene_component_2)))
  (`|ExecutionSequence`
    (:`then_0`
      (`SceneComponent.K2_SetRelativeRotation` _camera_scene_component_2 (`KismetMathLibrary.MakeRotator` (`self.CurrentRoll`) _relativerotation_pitch _relativerotation_yaw) false false)
      (set `self.OffsetPitch` (`KismetMathLibrary.Lerp` (`self.OffsetPitch`) 0.0 (* 10.0 (`GameplayStatics.GetWorldDeltaSeconds`))))
      (set `self.CurrentRoll` (`KismetMathLibrary.Lerp` (`self.CurrentRoll`) 0.0 (* 10.0 (`GameplayStatics.GetWorldDeltaSeconds`))))
      (bind _output_get (set `self.CurrentFOV` (`KismetMathLibrary.Lerp` (`self.CurrentFOV`) (`self.DefaultFOV`) (* 10.0 (`GameplayStatics.GetWorldDeltaSeconds`)))))
      (set `/Game/Main/Blueprints/DefaultGameMode/CM_CameraManager.FOV` _output_get (`self.CameraManager`)))
    (:`then_1`
      (set `self.BobAmplitude` (`KismetMathLibrary.Lerp` (`self.BobAmplitude`) 0.0 (* 4.0 (`GameplayStatics.GetWorldDeltaSeconds`))))
      (set `self.BobPhase` (mod (* (`KismetSystemLibrary.GetGameTimeInSeconds`) (`self.BobFreq`)) 1.0))
      (`SceneComponent.K2_SetRelativeLocation` _camera_scene_component (`KismetMathLibrary.MakeVector` _relativelocation_x _relativelocation_y (+ (.z (.location (`self.InitialTransform`))) (* (`CurveFloat.GetFloatValue` (`self.BobbingCurve`) (`self.BobPhase`)) (`self.BobAmplitude`)) (`self.OffsetPitch`))) false false))))

(fn `CalculateValueModify`
  (params (Input :type "Float (double-precision)") (Accel :type "Float (double-precision)") (Current :type "Float (double-precision)") (Max :type "Float (double-precision)"))
  (returns (ReturnValue :type "Float (double-precision)"))
  (return (`KismetMathLibrary.FClamp` (+ Current (* (* Accel (`KismetMathLibrary.SignOfFloat` Input)) (`GameplayStatics.GetWorldDeltaSeconds`))) (* Max -1.0) Max)))