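; Actor component that gives a door-like object open and close behavior by swinging an anchor component.
; Initialize supplies the anchor, while SetOpen and ToggleOpen change the IsOpen flag.
; Each Tick lerps the anchor's relative yaw toward the open or closed angle by Speed times delta time, giving an eased swing and leaving pitch and roll untouched.
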(event `self.ReceiveTick`
  (params (DeltaSeconds :type "Float (single-precision)"))
  (bind _dooranchor (`self.DoorAnchor`))
  (bind (_relativerotation_roll _relativerotation_pitch _relativerotation_yaw) (`KismetMathLibrary.BreakRotator` (`SceneComponent.RelativeRotation` _dooranchor)))
  (`SceneComponent.K2_SetRelativeRotation` _dooranchor (`KismetMathLibrary.MakeRotator` _relativerotation_roll _relativerotation_pitch (`KismetMathLibrary.Lerp` _relativerotation_yaw (`KismetMathLibrary.SelectFloat` (`self.OpenAngle`) (`self.ClosedAngle`) (`self.IsOpen`)) (* (`self.Speed`) (`GameplayStatics.GetWorldDeltaSeconds`)))) false false))

(fn `Initialize`
  (params (DoorAnchor :type "SceneComponent Object Reference"))
  (set `self.DoorAnchor` DoorAnchor))

(fn `SetOpen`
  (params (IsOpen :type Boolean))
  (set `self.IsOpen` IsOpen))

(fn `ToggleOpen`
  (set `self.IsOpen` (not (`self.IsOpen`))))