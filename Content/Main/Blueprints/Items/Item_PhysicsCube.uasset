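; Physics cube inventory item whose item-added event is empty, leaving all its logic disconnected so it never runs.
; The dormant graph grants GA_Test through the owner's Ability System Component when Quantity is at most one, storing the handle.
; It then waits for an Event.AbilityTriggered gameplay event carrying an A_PhysicsCube, removes the item from the Inventory and clears the ability once Quantity reaches zero.
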(event `self.OnItemAdded`
  (params (Item :type "ItemBase Object Reference") (InventoryContext :type "InventoryBase Object Reference") (InventoryOperation :type "InventoryOperationStruct Structure")))