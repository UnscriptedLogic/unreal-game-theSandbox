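; ItemFrag_Stackable is an item fragment that enforces a max stack size when an item is added to an inventory.
; It extends the parent's add check: when the existing slot is full, it searches the inventory's other items of that class, skipping the first match.
; The first one with room returns as an override slot (201); otherwise the response requests a new slot (202).
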(fn `Pass_ItemToBeAddedToInventory`
  (params (InventoryContext :type "InventoryBase Object Reference") (HasExistingSlot :type Boolean) (existingSlot :type "ItemBase Object Reference"))
  (returns (overrideSlot :type "ItemBase Object Reference") (ReturnValue :type "Response Structure"))
  (locals (Response :type "Response Structure") (Inventory :type "/Game/Main/Blueprints/Components/Inventory/Inventory Object Reference") (OtherSlots :type "Array of ItemBase Object Reference"))
  (bind _asinventory (cast `/Game/Main/Blueprints/Components/Inventory/Inventory` (`local.InventoryContext`)))
  (set `local.Inventory` _asinventory)
  (bind (_overrideslot _returnvalue) (`parent.Pass_ItemToBeAddedToInventory` InventoryContext HasExistingSlot existingSlot))
  (set `local.Response` _returnvalue)
  (`|ExecutionSequence`
    (:`then_0`
      (if (`local.HasExistingSlot`)
        (if (>= (`ItemBase.quantity` (`local.existingSlot`)) (`self.MaxStack`))
          (bind (_found _itemobjects) (`/Game/Main/Blueprints/Components/Inventory/Inventory.FindItemObjectsByType` (`local.Inventory`) (`GameplayStatics.GetObjectClass` (`local.existingSlot`))))
          (set `local.OtherSlots` _itemobjects)
          (`KismetArrayLibrary.Array_Remove` (`local.OtherSlots`))
          (if (> (`KismetArrayLibrary.Array_Length` (`local.OtherSlots`)) 0)
            (for _array_element (`local.OtherSlots`)
              (if (not (>= (`ItemBase.quantity` _array_element) (`self.MaxStack`)))
                (return _array_element (make `Response` 201 "Use Override Slot"))))
            (set `local.Response` (make `Response` 202 "New Slot Required"))
            (else
              (set `local.Response` (make `Response` 202 "New Slot Required")))))))
    (:`then_1`
      (return null (`local.Response`)))))