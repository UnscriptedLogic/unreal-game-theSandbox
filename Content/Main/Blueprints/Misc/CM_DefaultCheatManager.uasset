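; Cheat manager with debug commands for previewing UI widgets and testing the camera manager.
; UI commands spawn transitions, a screen-space widget and a sample tip pop-up, with delay events removing some afterwards.
; The circle transition binds a covered callback, and a transition-ready event adds a placeholder UI.
; Camera commands make CM_CameraManager claim or unclaim the root component of the first actor tagged CM_Reference.
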(event `OnSimpleTransitionReady_Event`
  (bind _returnvalue (`|CreateWidget` "/Game/Main/Widgets/PlaceHolder/UI_PlaceHolder.UI_PlaceHolder_C" (`GameplayStatics.GetPlayerController` 0)))
  (`UserWidget.AddToViewport` _returnvalue 0))

(event `DestroyPopUp`
  (params (Delay :type "Float (double-precision)") (Widget :type "/Game/Main/Widgets/TipPopUp/UI_TipPopUp Object Reference"))
  (`KismetSystemLibrary.Delay` Delay)
  (`/Game/Main/Widgets/TipPopUp/UI_TipPopUp.DestroySelf` Widget))

(event `RemoveWidgetAfterDelay`
  (params (Widget :type "Widget Object Reference") (Delay :type "Float (double-precision)"))
  (`KismetSystemLibrary.Delay` Delay)
  (`Widget.RemoveFromParent` Widget))

(fn `Camera_TestClaim`
  (locals (RefPoint :type "Actor Object Reference"))
  (bind _outactors (`GameplayStatics.GetAllActorsWithTag` "CM_Reference"))
  (if (> (`KismetArrayLibrary.Array_Length` _outactors) 0)
    (set `local.RefPoint` (`|GetArrayItem` _outactors))
    (`|ExecutionSequence`
      (:`then_0`
        (bind _ascm_camera_manager (cast `/Game/Main/Blueprints/DefaultGameMode/CM_CameraManager` (`GameplayStatics.GetPlayerCameraManager` 0)))
        (`/Game/Main/Blueprints/DefaultGameMode/CM_CameraManager.Claim` _ascm_camera_manager (`Actor.RootComponent` (`local.RefPoint`))))
      (:`then_1`))))

(fn `Camera_TestUnclaim`
  (locals (RefPoint :type "Actor Object Reference"))
  (bind _outactors (`GameplayStatics.GetAllActorsWithTag` "CM_Reference"))
  (if (> (`KismetArrayLibrary.Array_Length` _outactors) 0)
    (set `local.RefPoint` (`|GetArrayItem` _outactors))
    (`|ExecutionSequence`
      (:`then_0`
        (bind _ascm_camera_manager (cast `/Game/Main/Blueprints/DefaultGameMode/CM_CameraManager` (`GameplayStatics.GetPlayerCameraManager` 0)))
        (`/Game/Main/Blueprints/DefaultGameMode/CM_CameraManager.Unclaim` _ascm_camera_manager (`Actor.RootComponent` (`local.RefPoint`))))
      (:`then_1`))))

(fn `UI_CircleScaleIn`
  (bind _returnvalue (`|CreateWidget` "/Game/Tutorial/CircleTransition/WB_CircleTransition.WB_CircleTransition_C"))
  (`UserWidget.AddToViewport` _returnvalue 0)
  (`self.RemoveWidgetAfterDelay` _returnvalue 5.0))

(fn `UI_CreateSimpleTransitionWipe`
  (bind _returnvalue (`|CreateWidget` "/Game/Tutorial/WB_SimpleTransitionWipe.WB_SimpleTransitionWipe_C"))
  (`UserWidget.AddToViewport` _returnvalue 0))

(fn `UI_ScreenSpace`
  (bind _returnvalue (`|CreateWidget` "/Game/Main/Widgets/ScreenSpaceTest/UI_ScreenSpace.UI_ScreenSpace_C"))
  (`UserWidget.AddToViewport` _returnvalue 0))

(fn `UI_SquareScaleIn`
  (bind _returnvalue (`|CreateWidget` "/Game/Main/Widgets/Transition_SquareScale/WB_SquareScaleIn.WB_SquareScaleIn_C"))
  (`UserWidget.AddToViewport` _returnvalue 0)
  (`self.RemoveWidgetAfterDelay` _returnvalue 5.0))

(fn `UI_TipPopUp`
  (bind _returnvalue (`|CreateWidget` "/Game/Main/Widgets/TipPopUp/UI_TipPopUp.UI_TipPopUp_C" null "Special Award - A Grey Box" (struct :`R` 1.0 :`G` 0.267666 :`B` 0.191946 :`A` 1.0)))
  (`UserWidget.AddToViewport` _returnvalue 0)
  (`self.DestroyPopUp` 4.0 _returnvalue))

(fn `UI_TransitionCircle`
  (bind _returnvalue (`|CreateWidget` "/Game/Main/Widgets/TransitionOpen_CircleSimple/TransitionOpen_CircleSimple.TransitionOpen_CircleSimple_C" null (struct :`R` 0.006995 :`G` 0.006995 :`B` 0.006995 :`A` 1.0) (struct :`R` 1.0 :`G` 1.0 :`B` 1.0 :`A` 1.0) (struct :`R` 0.791667 :`G` 0.297926 :`A` 1.0) "\"MIHOYO UI\""))
  (add `/Game/Main/Widgets/TransitionOpen_CircleSimple/TransitionOpen_CircleSimple.Transition_Covered` _returnvalue (`|CreateDelegate` :!event `OnSimpleTransitionReady_Event`))
  (`UserWidget.AddToViewport` _returnvalue 1))