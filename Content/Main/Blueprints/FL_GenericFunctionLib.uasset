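; Generic Blueprint function library with helpers for pseudo-random procs, range remapping and tagged logging.
; PseudoRandomDistributor rolls against a chance from CalculatePRD that grows linearly with a by-ref try count, resetting it on a proc and incrementing otherwise.
; MapToRange linearly remaps a value between two ranges without clamping.
; PrintLog prefixes messages with level and bracketed gameplay tags, with screen and log output gated by CanLogOutput.
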(fn CalculatePRD
  (params (Tries :type Integer) (Chance :type Float%20%28double-precision%29))
  (return (/ (Math|Conversions|ToFloat(Integer) Tries) (/ 2.0 Chance))))

(fn PseudoRandomDistributor
  (params (Count :type Integer%20%28by%20ref%29) (Chance :type Float%20%28double-precision%29))
  (bind _returnvalue (CallFunction|CalculatePRD Count Chance))
  (LocalVariables|SetCalculatedChance _returnvalue)
  (if (<= (Math|Random|RandomFloat) _returnvalue)
    (|SetBy-RefVar Count)
    (return true (LocalVariables|GetCalculatedChance))
    (else
      (Math|Integer|IncrementInt Count
        (:%20%20
          (return false (LocalVariables|GetCalculatedChance)))))))

(fn MaptoRange
  (params (OutputRange :type Float%20Range%20Structure) (InputRange :type Float%20Range%20Structure) (Input :type Float%20%28double-precision%29))
  (bind (_lowerbound _upperbound) (Utilities|Struct|BreakFloatRange OutputRange))
  (bind (_lowerbound_2 _upperbound_2) (Utilities|Struct|BreakFloatRange InputRange))
  (return (|(output_start+(((output_end-output_start)/(input_end-input_start))*(input-input_start))) (.value _lowerbound) (.value _upperbound) (.value _upperbound_2) (.value _lowerbound_2) Input)))

(fn PrintLog
  (params (Context :type Object%20Object%20Reference) (String :type String) (Tags :type Gameplay%20Tag%20Container%20Structure) (Level :type ENotifyType%20Enum :default "NewEnumerator0"))
  (bind _canlogoutput (LocalVariables|GetCanLogOutput))
  (bind _gameplaytags (GameplayTags|BreakGameplayTagContainer Tags))
  (Utilities|FlowControl|Sequence
    (:then_0
      (if (> (Utilities|Array|Length _gameplaytags) 0)
        (for _array_element _gameplaytags
          (LocalVariables|SetTagString (Utilities|String|Append (LocalVariables|GetTagString) "[" (Utilities|String|ToString(Name) (GameplayTags|GetTagName _array_element)) "] ")))))
    (:then_1
      (Development|PrintString Context (Utilities|String|ToString(Text) (Utilities|Text|FormatText "<{Level}> {tags}| {string}" (Utilities|String|EnumtoString Level) (LocalVariables|GetTagString) String)) _canlogoutput _canlogoutput))))