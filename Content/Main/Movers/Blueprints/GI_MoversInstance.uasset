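; Game instance for Movers that handles multiplayer sessions and stores per-level scores.
; It uses Advanced Sessions to host a level as a listen server, join the first session found, or accept invites.
; A LevelData map holds each level's data, with score updates applied only to existing entries and logged.
; A debug function prints every level's stored score.
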(event `CreateSession`
  (params (bUseLAN :type Boolean) (Level :type "World Soft Object Reference"))
  (`CreateSessionCallbackProxyAdvanced.CreateAdvancedSession` :`PlayerController` (`GameplayStatics.GetPlayerController` 0) :`PublicConnections` 10 :`PrivateConnections` 10 :`bUseLAN` bUseLAN :`bUseLobbiesIfAvailable` false
    (:`OnSuccess`
      (`GameplayStatics.OpenLevelBySoftObjectPtr` Level true "?listen"))
    (:`OnFailure`
      (`KismetSystemLibrary.PrintString` "Could not start session"))))

(event `JoinSession`
  (params (bUseLAN :type Boolean))
  (bind _returnvalue (`GameplayStatics.GetPlayerController` 0))
  (bind _results (`FindSessionsCallbackProxyAdvanced.FindSessionsAdvanced` _returnvalue 100 bUseLAN "AllServers")
    (:`then`
      (`KismetSystemLibrary.PrintString` "Finding Sessions..."))
    (:`OnSuccess`
      (if (> (`KismetArrayLibrary.Array_Length` _results) 0)
        (`KismetSystemLibrary.PrintString` "Session Found")
        (`JoinSessionCallbackProxy.JoinSession` _returnvalue (`|GetArrayItem` _results)
          (:`OnSuccess`
            (`KismetSystemLibrary.PrintString` "Connected to session!"))
          (:`OnFailure`
            (`KismetSystemLibrary.PrintString` "Failed to connect to session")))
        (else
          (`KismetSystemLibrary.PrintString` "No Sessions Found"))))
    (:`OnFailure`
      (`KismetSystemLibrary.PrintString` "Failed to find sessions"))))

(event `self.OnSessionInviteAccepted`
  (params (LocalPlayerNum :type Integer) (PersonInvited :type "BPUniqueNetId Structure") (SessionToJoin :type "BlueprintSessionResult Structure (by ref)"))
  (`JoinSessionCallbackProxy.JoinSession` (`GameplayStatics.GetPlayerController` 0) SessionToJoin))

(fn `DEBUG_LogAllDataValues`
  (locals (CurrLevelData :type "/Game/Main/Movers/Blueprints/Structs/S_MoversLevelData Structure") (CurrLevelName :type String) (AllLevelDataString :type String))
  (bind _currleveldata_score (break `/Game/Main/Movers/Blueprints/Structs/S_MoversLevelData` (`local.CurrLevelData`)))
  (`|ExecutionSequence`
    (:`then_0`
      (bind _keys (`BlueprintMapLibrary.Map_Keys` (`self.LevelData`)))
      (for (_array_element _array_index) _keys
        (`|ExecutionSequence`
          (:`then_0`
            (set `local.CurrLevelName` _array_element)
            (bind _values (`BlueprintMapLibrary.Map_Values` (`self.LevelData`)))
            (set `local.CurrLevelData` (`|GetArrayItem` _values _array_index)))
          (:`then_1`
            (set `local.AllLevelDataString` (`KismetStringLibrary.Concat_StrStr` (`local.AllLevelDataString`) (`KismetTextLibrary.Conv_TextToString` (`|FormatText` "{Index} | {LevelName}: {LevelData} \n" (`local.CurrLevelName`) _currleveldata_score _array_index))))))))
    (:`then_1`
      (`/Game/Main/Blueprints/FL_GenericFunctionLib.PrintLog` null (`local.AllLevelDataString`)))))

(fn `SetLevelScore`
  (params (Level :type String) (Score :type Integer))
  (locals (LevelData :type "/Game/Main/Movers/Blueprints/Structs/S_MoversLevelData Structure"))
  (bind _level (`local.Level`))
  (bind (_value _returnvalue) (`BlueprintMapLibrary.Map_Find` (`self.LevelData`) (`local.Level`)))
  (if _returnvalue
    (bind _output_get (set `local.LevelData` _value))
    (bind _structout (setmembers `/Game/Main/Movers/Blueprints/Structs/S_MoversLevelData` :`StructRef` _output_get :`Score` (`local.Score`)))
    (`BlueprintMapLibrary.Map_Add` (`self.LevelData`) (`local.Level`) _structout)
    (`/Game/Main/Blueprints/FL_GenericFunctionLib.PrintLog` self (`KismetTextLibrary.Conv_TextToString` (`|FormatText` "Level Score Updated: \n{LevelName}: {Score}" _level (`.Score_5_7B5E0AB94D90B6A2336A37BD49C9DBCC` (break `/Game/Main/Movers/Blueprints/Structs/S_MoversLevelData` (`BlueprintMapLibrary.Map_Find` (`self.LevelData`) _level))))) (struct :`GameplayTags` (struct :`(TagName` "Debug.System.Architecture.GameInstance"))) "NewEnumerator1")
    (else
      (`/Game/Main/Blueprints/FL_GenericFunctionLib.PrintLog` self (`KismetStringLibrary.Concat_StrStr` "Level Does Not Exist" (`local.Level`)) (struct :`GameplayTags` (struct :`(TagName` "Debug.System.Architecture.GameInstance"))) "NewEnumerator1"))))