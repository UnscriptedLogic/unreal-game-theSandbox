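; BP_MoversMain is a locally controlled pawn that provides a test front end for hosting or joining Movers multiplayer sessions.
; BeginPlay caches the GI_MoversInstance game instance, then, for local control only, shows the mouse cursor and adds the WB_TestServerHost widget with create and join callbacks bound.
; OnCreateSession and OnJoinSession forward the LAN choice to the game instance, with creation targeting the MoversLobby level.
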(event `self.ReceiveBeginPlay`
  (`|ExecutionSequence`
    (:`then_0`
      (`self.TryInitializeGameInstance`))
    (:`then_1`
      (if (`self.IsLocallyControlled`)
        (`self.BeginPlay_Local`)
        (else
          (`KismetSystemLibrary.PrintString` "Not locally controlled"))))))

(event `BeginPlay_Local`
  (`|ExecutionSequence`
    (:`then_0`
      (set `PlayerController.bShowMouseCursor` true (`GameplayStatics.GetPlayerController` 0)))
    (:`then_1`
      (bind _returnvalue (`|CreateWidget` "/Game/Main/ClassroomPurgatory/Blueprints/Widgets/WB_TestServerHost.WB_TestServerHost_C"))
      (`UserWidget.AddToViewport` _returnvalue 0)
      (add `/Game/Main/ClassroomPurgatory/Blueprints/Widgets/WB_TestServerHost.OnCreateSessionClicked` _returnvalue (`|CreateDelegate` :!event `OnCreateSession`))
      (add `/Game/Main/ClassroomPurgatory/Blueprints/Widgets/WB_TestServerHost.OnJoinSessionClicked` _returnvalue (`|CreateDelegate` :!event `OnJoinSession`)))))

(fn `OnCreateSession`
  (params (bUseLAN :type Boolean))
  (`/Game/Main/Movers/Blueprints/GI_MoversInstance.CreateSession` (`self.GameInstance`) bUseLAN "/Game/Main/Movers/MoversLobby.MoversLobby"))

(fn `OnJoinSession`
  (params (bUseLAN :type Boolean))
  (`/Game/Main/Movers/Blueprints/GI_MoversInstance.JoinSession` (`self.GameInstance`) bUseLAN))

(fn `TryInitializeGameInstance`
  (bind _returnvalue (`GameplayStatics.GetGameInstance`))
  (`/Engine/EditorBlueprintResources/StandardMacros.IsValid` (`self.GameInstance`)
    (:`Is Not Valid`
      (bind _asgi_movers_instance (cast `/Game/Main/Movers/Blueprints/GI_MoversInstance` _returnvalue)
        (:`then`
          (set `self.GameInstance` _asgi_movers_instance))
        (:`CastFailed`
          (`/Game/Main/Blueprints/FL_GenericFunctionLib.PrintLog` null (`KismetStringLibrary.Concat_StrStr` "Could not cast to game instance from: " (`KismetSystemLibrary.GetDisplayName` _returnvalue)) (struct :`GameplayTags` (struct :`(TagName` "Debug.Entities.Player"))) "NewEnumerator2"))))))

(fn `UserConstructionScript`)