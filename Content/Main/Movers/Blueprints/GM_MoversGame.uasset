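; Game mode for the Movers furniture-delivery match, running it from player join to the return to the lobby.
; Logins and logouts update the player list in GS_Movers, and play starts once the count expected by GI_MoversInstance connects.
; Buttons tagged SubmitDelivery are bound at BeginPlay; submission scores the summed health of deliverable furniture from the objective handler.
; It then changes game state and server-travels to the lobby after a delay; a separate event restarts the map.
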(event `self.ReceiveBeginPlay`
  (`|ExecutionSequence`
    (:`then_0`
      (`self.InitializeGameMode`))
    (:`then_1`
      (`self.InitializeDeliverySubmit`))))

(event `OnSubmitDeliver_Event`
  (`|ExecutionSequence`
    (:`then_0`
      (bind _outactors (`GameplayStatics.GetAllActorsOfClass` "/Game/Main/Movers/Blueprints/A_FurnitureObjectiveHandler.A_FurnitureObjectiveHandler_C"))
      (if (> (`KismetArrayLibrary.Array_Length` _outactors) 0)
        (set `/Game/Main/Movers/Blueprints/GS_Movers.Score` (`self.CalculateHPSum` (`|GetArrayItem` _outactors)) (`self.GS_Movers`))))
    (:`then_1`
      (`/Game/Main/Movers/Blueprints/GS_Movers.ChangeState` (`self.GS_Movers`) "NewEnumerator2")
      (`KismetSystemLibrary.Delay` 5.0)
      (`AdvancedSessionsLibrary.ServerTravel` "/Game/Main/Movers/MoversLobby?listen"))))

(event `self.K2_PostLogin`
  (params (NewPlayer :type "PlayerController Object Reference"))
  (bind _numberofplayers (`/Game/Main/Movers/Blueprints/GI_MoversInstance.NumberOfPlayers` (`self.GI_Movers`)))
  (bind _returnvalue (`KismetArrayLibrary.Array_Length` (`/Game/Main/Movers/Blueprints/GS_Movers.ConnectedPlayers` (`self.GS_Movers`))))
  (`self.InitializeGameState`)
  (`self.InitializeGameInstance`)
  (`/Game/Main/Movers/Blueprints/GS_Movers.TryAddPlayer` (`self.GS_Movers`) NewPlayer)
  (`KismetSystemLibrary.PrintString` (`KismetTextLibrary.Conv_TextToString` (`|FormatText` "Expected Players: {expected} | Current Players: {current}" _numberofplayers _returnvalue)))
  (if (>= _returnvalue _numberofplayers)
    (`/Game/Main/Movers/Blueprints/GS_Movers.ChangeState` (`self.GS_Movers`) "NewEnumerator1")
    (`KismetSystemLibrary.PrintString` "In Play!")))

(event `self.K2_OnLogout`
  (params (ExitingController :type "Controller Object Reference"))
  (`self.InitializeGameState`)
  (`/Game/Main/Movers/Blueprints/GS_Movers.TryRemovePlayer` (`self.GS_Movers`) ExitingController))

(event `Server_RestartMap`
  (bind _returnvalue (`AdvancedSessionsLibrary.ServerTravel` "/Game/Main/Movers/MoversGame?listen"))
  (`KismetSystemLibrary.PrintString` (`KismetStringLibrary.Conv_BoolToString` _returnvalue)))

(fn `CalculateHPSum`
  (params (ObjectiveHandler :type "/Game/Main/Movers/Blueprints/A_FurnitureObjectiveHandler Object Reference"))
  (returns (HealthSum :type Integer))
  (locals (Sum :type Integer :default 0))
  (`|ExecutionSequence`
    (:`then_0`
      (for _array_element (`.Furniture` (`/Game/Main/Movers/Blueprints/A_FurnitureObjectiveHandler.CalculateDeliverables` (`local.ObjectiveHandler`)))
        (set `local.Sum` (+ (`local.Sum`) (`/Game/Main/Movers/Blueprints/Items/A_Furniture.Health` _array_element)))))
    (:`then_1`
      (return (`local.Sum`)))))

(fn `InitializeDeliverySubmit`
  (locals (Submitters :type "Array of Actor Object Reference"))
  (`|ExecutionSequence`
    (:`then_0`
      (bind _outactors (`GameplayStatics.GetAllActorsWithTag` "SubmitDelivery"))
      (set `local.Submitters` _outactors)
      (if (> (`KismetArrayLibrary.Array_Length` _outactors) 0)
        (for _array_element (`local.Submitters`)
          (bind _asa_button (cast `/Game/Main/Blueprints/Items/Button/A_Button` _array_element))
          (add `/Game/Main/Blueprints/Items/Button/A_Button.ButtonPressed` _asa_button (`|CreateDelegate` :!event `OnSubmitDeliver_Event`)))
        (else
          (`/Game/Main/Blueprints/FL_GenericFunctionLib.PrintLog` null "No Delivery Submit Foud" (struct) "NewEnumerator2"))))))

(fn `InitializeGameInstance`
  (`/Engine/EditorBlueprintResources/StandardMacros.IsValid` (`self.GI_Movers`)
    (:`Is Not Valid`
      (bind _asgi_movers_instance (cast `/Game/Main/Movers/Blueprints/GI_MoversInstance` (`GameplayStatics.GetGameInstance`)))
      (set `self.GI_Movers` _asgi_movers_instance))))

(fn `InitializeGameMode`
  (`|ExecutionSequence`
    (:`then_0`
      (`self.InitializeGameState`))
    (:`then_1`
      (`self.InitializeGameInstance`))))

(fn `InitializeGameState`
  (`/Engine/EditorBlueprintResources/StandardMacros.IsValid` (`self.GS_Movers`)
    (:`Is Not Valid`
      (bind _asgs_movers (cast `/Game/Main/Movers/Blueprints/GS_Movers` (`GameplayStatics.GetGameState`)))
      (set `self.GS_Movers` _asgs_movers))))

(fn `UserConstructionScript`)