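; Gameplay ability that conjures a volley of A_Rock "fireballs" in front of the avatar, then launches them.
; Random positions around the CameraRef arrow feed a delayed loop that spawns rocks and tweens them into place, scale and rotation.
; A second staggered loop sets velocities from AC_InteractionComponent's camera-centre trace, falling back to arrow forward.
; Each launch stretches the rock with shockwave VFX and camera shake, and the ability ends afterwards.
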(event `self.K2_ActivateAbility`
  (bind _returnvalue (`self.GetAvatarActorFromActorInfo`))
  (bind _returnvalue_2 (`Actor.GetComponentByClass` _returnvalue "/Game/Main/Blueprints/Components/Interaction/AC_InteractionComponent.AC_InteractionComponent_C"))
  (bind _output (`|GetArrayItem` (`Actor.GetComponentsByTag` (`self.GetAvatarActorFromActorInfo`) "/Script/Engine.ArrowComponent" "CameraRef")))
  (bind _output_2 (`|GetArrayItem` (`Actor.GetComponentsByTag` (`self.GetAvatarActorFromActorInfo`) "/Script/Engine.ArrowComponent" "CameraRef")))
  (bind (_bblockinghit _binitialoverlap _time _distance _location _impactpoint _normal _impactnormal _physmat _hitactor _hitcomponent _hitbonename _bonename _hititem _elementindex _faceindex _tracestart _traceend) (`GameplayStatics.BreakHitResult` (`.OutHit` (`/Game/Main/Blueprints/Components/Interaction/AC_InteractionComponent.GetCenterOfCamera` :`self` _returnvalue_2 :`OverrideRange` 9999.0))))
  (`|ExecutionSequence`
    (:`then_0`
      (for _ (range (+ (`self.Amount`) 1))
        (`KismetArrayLibrary.Array_Add` (`self.Positions`) (+ (`SceneComponent.K2_GetComponentLocation` _output_2) (* (`SceneComponent.GetForwardVector` _output_2) 400.0) (* (`SceneComponent.GetRightVector` _output_2) (`KismetMathLibrary.RandomFloatInRange` -600.0 600.0)) (* (`SceneComponent.GetUpVector` _output_2) (`KismetMathLibrary.RandomFloatInRange` 100.0 300.0))))))
    (:`then_1`
      (bind _index (`/Game/Main/Blueprints/ML_GenericMacroLib.ForLoopWithDelay` 0 (`self.Amount`) 0.1)
        (:`Loop Body`
          (bind _returnvalue_3 (`|SpawnActorFromClass` "/Game/Main/InvokerTest/A_Rock.A_Rock_C" (`KismetMathLibrary.MakeTransform` (+ (`SceneComponent.K2_GetComponentLocation` _output) (* (`SceneComponent.GetForwardVector` _output) 200.0)) (struct) (0.0 0.0 0.0)) "Undefined" "MultiplyWithRoot" null null))
          (`Actor.SetLifeSpan` _returnvalue_3 12.0)
          (`KismetArrayLibrary.Array_Add` (`self.Fireballs`) _returnvalue_3)
          (bind _output_3 (`|GetArrayItem` (`self.Positions`) _index))
          (bind _returnvalue_4 (`KismetStringLibrary.Concat_StrStr` (`KismetSystemLibrary.GetDisplayName` _returnvalue_3) (`KismetStringLibrary.Conv_IntToString` _index) (`KismetStringLibrary.Conv_VectorToString` _output_3)))
          (`XiTweenUtil.TweenActorMoveSync` (`KismetStringLibrary.Concat_StrStr` _returnvalue_4 "Move") 0.25 _returnvalue_3 _output_3 "OutSine")
          (`XiTweenUtil.TweenActorScaleSync` (`KismetStringLibrary.Concat_StrStr` _returnvalue_4 "Scale") 0.25 _returnvalue_3 (1.0 1.0 1.0) "OutBack")
          (`XiTweenUtil.TweenActorRotationSync` (`KismetStringLibrary.Concat_StrStr` _returnvalue_4 "Rotation") 0.3 _returnvalue_3 (`KismetMathLibrary.RandomRotator` true) "OutSine"))
        (:`Completed`
          (`KismetSystemLibrary.Delay` 0.2)
          (bind _index_2 (`/Game/Main/Blueprints/ML_GenericMacroLib.ForLoopWithDelay` 0 (- (`KismetArrayLibrary.Array_Length` (`self.Fireballs`)) 1) 0.1)
            (:`Loop Body`
              (`|ExecutionSequence`
                (:`then_0`
                  (`/Engine/EditorBlueprintResources/StandardMacros.IsValid` _returnvalue_2
                    (:`Is Valid`
                      (bind _output_4 (`|GetArrayItem` (`self.Fireballs`) _index_2))
                      (bind _projectilemovement (`/Game/Main/InvokerTest/A_Rock.ProjectileMovement` _output_4))
                      (set `MovementComponent.Velocity` (+ _tracestart (* (`KismetMathLibrary.Normal` (- (`KismetMathLibrary.SelectVector` _impactpoint _traceend _bblockinghit) (`Actor.K2_GetActorLocation` _output_4))) (`self.Speed`))) _projectilemovement))
                    (:`Is Not Valid`
                      (set `MovementComponent.Velocity` (* (`SceneComponent.GetForwardVector` (`|GetArrayItem` (`Actor.GetComponentsByTag` _returnvalue "/Script/Engine.ArrowComponent" "CameraRef"))) (`self.Speed`)) _projectilemovement))))
                (:`then_1`
                  (bind _velocity (`MovementComponent.Velocity` _projectilemovement))
                  (`Actor.K2_SetActorRotation` _output_4 (`KismetMathLibrary.Conv_VectorToRotator` _velocity) false)
                  (`XiTweenUtil.TweenActorScaleSync` (`KismetStringLibrary.Concat_StrStr` "FireBallMoveScale" (`KismetStringLibrary.Conv_IntToString` _index_2)) 0.15 _output_4 (3.0 0.5 0.5) "OutExpo")
                  (bind _returnvalue_5 (`Actor.K2_GetActorLocation` _output_4))
                  (`NiagaraFunctionLibrary.SpawnSystemAtLocation` "/Game/Main/InvokerTest/NS_KickShockwave.NS_KickShockwave" _returnvalue_5 (`KismetMathLibrary.Conv_VectorToRotator` (* _velocity -1.0)))
                  (`GameplayStatics.PlayWorldCameraShake` "/Game/Main/InvokerTest/CS_RumbleShake.CS_RumbleShake_C" _returnvalue_5 0.0 1000.0))))
            (:`Completed`
              (`self.K2_EndAbility`))))))))