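; GA_ShotgunAir is a gameplay ability that fires an air shotgun by spawning an A_ShotgunAir actor.
; On activation it builds a GE_ImpactEffect spec with the avatar as instigator and causer, setting Data.Damage by caller from Magnitude.
; The actor receives that spec and spawns just ahead of the avatar, aimed along its CameraRef-tagged arrow component.
; The graph never calls CommitAbility or EndAbility.
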(event `self.K2_ActivateAbility`
  (bind _returnvalue (`self.GetAvatarActorFromActorInfo`))
  (bind _returnvalue_2 (`self.GetAvatarActorFromActorInfo`))
  (bind _returnvalue_3 (`AbilitySystemBlueprintLibrary.MakeSpecHandleByClass` "/Game/Main/InvokerTest/Abilities/FireBarrage/GE_ImpactEffect.GE_ImpactEffect_C" _returnvalue _returnvalue))
  (bind _returnvalue_4 (`AbilitySystemBlueprintLibrary.AssignTagSetByCallerMagnitude` _returnvalue_3 (struct :`TagName` "Data.Damage") (`self.Magnitude`)))
  (`|SpawnActorFromClass` "/Game/Main/InvokerTest/Abilities/AirShotgun/A_ShotgunAir.A_ShotgunAir_C" (`KismetMathLibrary.MakeTransform` (+ (`Actor.K2_GetActorLocation` _returnvalue_2) (* (`Actor.GetActorForwardVector` _returnvalue_2) 50.0) (0.0 0.0 0.0)) (`KismetMathLibrary.Conv_VectorToRotator` (`SceneComponent.GetForwardVector` (`|GetArrayItem` (`Actor.GetComponentsByTag` _returnvalue_2 "/Script/Engine.ArrowComponent" "CameraRef"))))) "AlwaysSpawn" "MultiplyWithRoot" null _returnvalue_4 (cast `Pawn` (`self.GetAvatarActorFromActorInfo`) :!pure true)))