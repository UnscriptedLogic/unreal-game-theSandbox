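; Actor component that gives its owner hit feedback when health changes, with pop-up damage numbers, a flash and a bounce.
; A GAS attribute-change listener on the owner drives the health event, which spawns A_DamageText showing the value delta.
; The event also briefly applies a flash overlay material to the owner's static mesh and tweens its scale from a stretch back to the original with an OutBack ease.
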(event `self.ReceiveBeginPlay`
  (`self.Initialize`))

(event `Initialize`
  (`|ExecutionSequence`
    (:`then_0`
      (set `self.StaticMeshRef` (`Actor.GetComponentByClass` (`self.GetOwner`) "/Script/Engine.StaticMeshComponent"))
      (set `self.OriginalScale` (`SceneComponent.RelativeScale3D` (`self.StaticMeshRef`))))
    (:`then_1`
      (bind (_asynctaskproxy _attribute _newvalue _oldvalue) (`AbilityAsync_WaitAttributeChanged.WaitForAttributeChanged` (`self.GetOwner`) (struct :`AttributeName` "Health" :`Attribute` "/Script/TheSandbox.BasicAttributeSet:Health" :`AttributeOwner` "/Script/CoreUObject.Class'/Script/TheSandbox.BasicAttributeSet'"))
        (:`Changed`
          (`self.OnHealthChanged_Event` _newvalue _oldvalue))))))

(event `OnHealthChanged_Event`
  (params (NewValue :type "Float (double-precision)") (OldValue :type "Float (double-precision)"))
  (`|ExecutionSequence`
    (:`then_0`
      (`|SpawnActorFromClass` "/Game/Main/InvokerTest/A_DamageText.A_DamageText_C" (`KismetMathLibrary.MakeTransform` (`Actor.K2_GetActorLocation` (`self.GetOwner`))) "Undefined" "MultiplyWithRoot" null (- NewValue OldValue) null))
    (:`then_1`
      (`MeshComponent.SetOverlayMaterial` (`self.StaticMeshRef`) "/Game/Main/InvokerTest/MO_DamageFlash.MO_DamageFlash")
      (`KismetSystemLibrary.Delay` 0.2)
      (`MeshComponent.SetOverlayMaterial` (`self.StaticMeshRef`) null))
    (:`then_2`
      (bind _returnvalue (`XiTweenUtil.TweenVector3DSync` (`KismetStringLibrary.Concat_StrStr` "MeshBounce" (`KismetSystemLibrary.GetDisplayName` (`self.StaticMeshRef`))) 0.25 (+ (`SceneComponent.RelativeScale3D` (`self.StaticMeshRef`)) (-0.25 -0.25 1.0)) (`self.OriginalScale`) "OutBack"))
      (add `XiTweenVector3D.OnUpdate` _returnvalue (delegate `UpdateEvent_MeshScale`)))))

(event `UpdateEvent_MeshScale`
  (params (curValue :type "Vector Structure"))
  (`SceneComponent.SetRelativeScale3D` (`self.StaticMeshRef`) curValue))