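; Gameplay ability that raises a boulder wall from the aimed surface and throws nearby objects and characters.
; After the player confirms the placement preview, a camera-center trace from the interaction component, not the target data, places the wall slightly inside the surface.
; A tween lifts it along world up with camera shake.
; Shortly into the rise, a box overlap pushes physics meshes and launches characters using the surface normal, then the ability ends.
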(event `self.K2_ActivateAbility`
  (bind _returnvalue (`Actor.GetComponentByClass` (`self.GetAvatarActorFromActorInfo`) "/Game/Main/Blueprints/Components/Interaction/AC_InteractionComponent.AC_InteractionComponent_C"))
  (bind (_bblockinghit _hitactor _outhit) (`/Game/Main/Blueprints/Components/Interaction/AC_InteractionComponent.GetCenterOfCamera` :`self` _returnvalue :`DrawDebugType` "ForOneFrame"))
  (bind (_bblockinghit_2 _binitialoverlap _time _distance _location _impactpoint _normal _impactnormal) (`GameplayStatics.BreakHitResult` _outhit))
  (`AbilityTask_WaitTargetData.WaitTargetData` "None" "UserConfirmed" "/Game/Main/InvokerTest/GTA_BoulderWallTarget.GTA_BoulderWallTarget_C" "/Game/Main/InvokerTest/A_BoulderWall.A_BoulderWall_C" "/Game/Main/Materials/M_IntersectMat_Inst.M_IntersectMat_Inst" 0.0 0.0 900.0 (struct :`Name` "BlockAll") true (`self.MakeTargetLocationInfoFromOwnerActor`) (struct) "/Script/GameplayAbilities.GameplayAbilityWorldReticle_ActorVisualization"
    (:`ValidData`
      (`|ExecutionSequence`
        (:`then_0`
          (`/Engine/EditorBlueprintResources/StandardMacros.IsValid` _returnvalue
            (:`Is Valid`
              (`KismetSystemLibrary.PrintString` "Hello")
              (if _bblockinghit
                (`|ExecutionSequence`
                  (:`then_0`
                    (set `self.Normal` _impactnormal)
                    (bind _returnvalue_2 (`|SpawnActorFromClass` "/Game/Main/InvokerTest/A_BoulderWall.A_BoulderWall_C" (`KismetMathLibrary.MakeTransform` (+ _impactpoint (* _impactnormal -100.0)) (`Actor.K2_GetActorRotation` (`self.GetAvatarActorFromActorInfo`))) "AlwaysSpawn" "MultiplyWithRoot" null null))
                    (set `self.SpawnedBoulder` _returnvalue_2)
                    (`XiTweenUtil.TweenActorMoveSync` "TweenBoulderMove" 0.25 _returnvalue_2 (+ (`Actor.K2_GetActorLocation` _returnvalue_2) (* (0.0 0.0 1.0) 300.0)) "OutSine")
                    (`KismetSystemLibrary.Delay` 0.1)
                    (`self.OnBoulderMoveFinish`))
                  (:`then_1`
                    (`GameplayStatics.PlayWorldCameraShake` "/Game/Main/InvokerTest/CS_RumbleShake.CS_RumbleShake_C" (`Actor.K2_GetActorLocation` (`self.SpawnedBoulder`)) 100.0 1000.0)))))))))))

(event `OnBoulderMoveFinish`
  (bind (_normal_x _normal_y _normal_z) (`KismetMathLibrary.BreakVector` (`self.Normal`)))
  (`|ExecutionSequence`
    (:`then_0`
      (bind (_outactors _returnvalue) (`KismetSystemLibrary.BoxOverlapActors` (`Actor.K2_GetActorLocation` (`self.SpawnedBoulder`)) (150.0 150.0 300.0) (`|MakeArray` "ObjectTypeQuery2" "ObjectTypeQuery3" :!type "EObjectTypeQuery Enum")))
      (`KismetSystemLibrary.PrintString` (`KismetStringLibrary.Conv_IntToString` (`KismetArrayLibrary.Array_Length` _outactors)))
      (if _returnvalue
        (for _array_element _outactors
          (`|ExecutionSequence`
            (:`then_0`
              (bind _returnvalue_2 (`Actor.GetComponentByClass` _array_element "/Script/Engine.StaticMeshComponent"))
              (if (`SceneComponent.IsSimulatingPhysics` _returnvalue_2 "None")
                (`PrimitiveComponent.AddForce` _returnvalue_2 (* (`self.Normal`) (`self.UpheaveForce`)) "None" true)))
            (:`then_1`
              (bind _ascharacter (cast `Character` _array_element))
              (`Character.LaunchCharacter` _ascharacter (* (`KismetMathLibrary.MakeVector` (* _normal_x 4.0) (* _normal_y 4.0) (`KismetMathLibrary.FClamp` _normal_z 1.0)) (`self.UpheaveForce`)) false false))))))
    (:`then_1`
      (`self.K2_EndAbility`))))