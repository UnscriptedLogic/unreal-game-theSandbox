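; Cheat class for the ClassroomPurgatory game mode that exposes a command to try starting the game.
; CMDTryStartGame forwards the request to TryStartGame on the PC_ClassroomPurgatory player controller.
; LoadController lazily casts and caches that controller, stopping if the cast fails.
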(fn `CMD_TryStartGame`
  (bind _as_pc_classroom_purgatory (`self.LoadController`))
  (`/Game/Main/ClassroomPurgatory/Blueprints/PC_ClassroomPurgatory.TryStartGame` _as_pc_classroom_purgatory))

(fn `LoadController`
  (returns (`As PC Classroom Purgatory` :type "/Game/Main/ClassroomPurgatory/Blueprints/PC_ClassroomPurgatory Object Reference"))
  (`|ExecutionSequence`
    (:`then_0`
      (`/Engine/EditorBlueprintResources/StandardMacros.IsValid` (`self.As PC Classroom Purgatory`)
        (:`Is Not Valid`
          (bind _aspc_classroom_purgatory (cast `/Game/Main/ClassroomPurgatory/Blueprints/PC_ClassroomPurgatory` (`self.GetPlayerController`)))
          (set `self.As PC Classroom Purgatory` _aspc_classroom_purgatory))))
    (:`then_1`
      (return (`self.As PC Classroom Purgatory`)))))