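; PC_ClassroomPurgatory is the player controller for the ClassroomPurgatory part of the game, setting up player input.
; On BeginPlay it logs its name and, for the local controller only, adds the IMC_Default Enhanced Input mapping context.
; Possessing a pawn enables that pawn's input for this controller, and unpossessing it disables that input.
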(event `self.ReceiveBeginPlay`
  (`KismetSystemLibrary.PrintString` (`KismetStringLibrary.Concat_StrStr` "[INFO] BeginPlay > " (`KismetSystemLibrary.GetDisplayName` self)))
  (`|ExecutionSequence`
    (:`then_0`
      (if (`self.IsLocalController`)
        (`EnhancedInputSubsystemInterface.AddMappingContext` (subsystem `EnhancedInputLocalPlayerSubsystem`) "/Game/Main/Blueprints/FirstPerson/IMC_Default.IMC_Default" 0 (struct))))))

(event `self.ReceivePossess`
  (params (PossessedPawn :type "Pawn Object Reference"))
  (`self.EnableInput` PossessedPawn self))

(event `self.ReceiveUnPossess`
  (params (UnpossessedPawn :type "Pawn Object Reference"))
  (`self.DisableInput` UnpossessedPawn self))

(fn `UserConstructionScript`)