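; GM_ClassroomPurgatoryGame is the game mode for the Classroom Purgatory game, tracking which player controllers are connected.
; PostLogin adds each new controller to the ConnectedPlayers list on GS_Classroom, and OnLogout removes it.
; CheckLoadGameState lazily casts and caches the game state on BeginPlay and before each change, reporting whether it is valid.
; Duplicate logins, unknown logouts and an invalid game state print error messages.
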(event `self.ReceiveBeginPlay`
  (`self.CheckLoadGameState`))

(event `self.K2_PostLogin`
  (params (NewPlayer :type "PlayerController Object Reference"))
  (bind _connectedplayers (`/Game/Main/ClassroomPurgatory/GS_Classroom.ConnectedPlayers` (`self.ClassroomGameState`)))
  (bind _isvalid (`self.CheckLoadGameState`))
  (if _isvalid
    (if (== (`KismetArrayLibrary.Array_Find` _connectedplayers NewPlayer) -1)
      (`KismetArrayLibrary.Array_Add` _connectedplayers NewPlayer)
      (else
        (`KismetSystemLibrary.PrintString` "[ERROR] The same controller was logged in twice somehow???")))
    (else
      (`KismetSystemLibrary.PrintString` "[ERROR] GameState is Invalid on LogIn"))))

(event `self.K2_OnLogout`
  (params (ExitingController :type "Controller Object Reference"))
  (bind _connectedplayers (`/Game/Main/ClassroomPurgatory/GS_Classroom.ConnectedPlayers` (`self.ClassroomGameState`)))
  (bind _isvalid (`self.CheckLoadGameState`))
  (if _isvalid
    (if (!= (`KismetArrayLibrary.Array_Find` _connectedplayers ExitingController) -1)
      (`KismetArrayLibrary.Array_RemoveItem` _connectedplayers ExitingController)
      (else
        (`KismetSystemLibrary.PrintString` "[ERROR] A controller that doesn't exist has tried to log out")))
    (else
      (`KismetSystemLibrary.PrintString` "[ERROR] GameState is Invalid on LogOut"))))

(fn `CheckLoadGameState`
  (returns (IsValid :type Boolean))
  (`|ExecutionSequence`
    (:`then_0`
      (`/Engine/EditorBlueprintResources/StandardMacros.IsValid` (`self.ClassroomGameState`)
        (:`Is Not Valid`
          (bind _asgs_classroom (cast `/Game/Main/ClassroomPurgatory/GS_Classroom` (`GameplayStatics.GetGameState`)))
          (set `self.ClassroomGameState` _asgs_classroom))))
    (:`then_1`
      (return (`KismetSystemLibrary.IsValid` (`self.ClassroomGameState`))))))

(fn `UserConstructionScript`)